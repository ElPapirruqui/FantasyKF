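; BP_MageShot is a mage shot actor that damages players it touches with a strong-stagger hit.
; On server authority, a sphere overlap calls OnDamaged on a BP_Player and destroys the shot whatever it overlapped, while a blocking hit only destroys it.
; The Destroyed event spawns a half-scale hit effect at the actor's location without an authority check, keeping the visual separate from the server-only damage logic.
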(event `self.ReceiveDestroyed`
  (`GameplayStatics.SpawnEmitterAtLocation` (`self.hitFx`) (`self.K2_GetActorLocation`) (struct) (0.5 0.5 0.5)))

(event `self.Sphere.OnComponentBeginOverlap`
  (params (OverlappedComponent :type "PrimitiveComponent Object Reference") (OtherActor :type "Actor Object Reference") (OtherComp :type "PrimitiveComponent Object Reference") (OtherBodyIndex :type Integer) (bFromSweep :type Boolean) (SweepResult :type "HitResult Structure (by ref)"))
  (`/Engine/EditorBlueprintResources/ActorMacros.Switch Has Authority`
    (:`Authority`
      (bind _asbp_player (cast `/Game/FantasyKF/Player/BP_Player` OtherActor)
        (:`then`
          (`/Game/FantasyKF/Player/BP_Player.BP_OnDamaged` _asbp_player 25.0 "Strong"))
        (:`CastFailed`
          _))
      (`self.K2_DestroyActor`))))

(event `self.Sphere.OnComponentHit`
  (params (HitComponent :type "PrimitiveComponent Object Reference") (OtherActor :type "Actor Object Reference") (OtherComp :type "PrimitiveComponent Object Reference") (NormalImpulse :type "Vector Structure") (Hit :type "HitResult Structure (by ref)"))
  (`/Engine/EditorBlueprintResources/ActorMacros.Switch Has Authority`
    (:`Authority`
      (`self.K2_DestroyActor`))))

(fn `UserConstructionScript`)